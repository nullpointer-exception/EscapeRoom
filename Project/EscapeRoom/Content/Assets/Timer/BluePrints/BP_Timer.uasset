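; Countdown timer actor that shows minutes and seconds remaining until game over on two text displays.
; Tick refreshes both displays, then uses a one-second Delay to pace CountdownMinute, which decrements seconds and rolls over into minutes.
; The zero check only returns, so no game-over action fires here.
; An Update_Clock event for real clock time remains, but its looping timer setup is disconnected.
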(event Custom|Update_Clock
  (bind _returnvalue (Math|DateTime|Now))
  ;[1 1 1] RealTimeClock
  (Rendering|Components|TextRender|SetText (Variables|Default|GetMinutes) (Utilities|Text|ToText(Integer) (Class|KismetMathLibrary|GetMinute _returnvalue)))
  (Rendering|Components|TextRender|SetText (Variables|Default|GetSeconds) (Utilities|Text|ToText(Integer) (Class|KismetMathLibrary|GetHour12 _returnvalue))))

(event EventTick
  (params (DeltaSeconds :type Float%20%28single-precision%29))
  (CallFunction|SetTimer)
  (Utilities|FlowControl|Delay 1.0)
  (CallFunction|CountdownMinute))

(event EventBeginPlay
  ;[1 1 1] RealTimeClock
)

(fn ConstructionScript)

(fn CountdownSeconds
  (bind _output_get (Variables|Default|SetTimeToGameOverSecond (- (Variables|Default|GetTimeToGameOverSecond) 1)))
  (Rendering|Components|TextRender|SetText (Variables|Default|GetSeconds) (Utilities|Text|ToText(Integer) _output_get))
  (return))

(fn CountdownMinute
  (CallFunction|CountdownSeconds)
  (if (< (Variables|Default|GetTimeToGameOverSecond) 0)
    (bind _output_get (Variables|Default|SetTimeToGameOverMinute (- (Variables|Default|GetTimeToGameOverMinute) 1)))
    (Rendering|Components|TextRender|SetText (Variables|Default|GetMinutes) (Utilities|Text|ToText(Integer) _output_get))
    (bind _output_get_2 (Variables|Default|SetTimeToGameOverSecond 59))
    (Rendering|Components|TextRender|SetText (Variables|Default|GetSeconds) (Utilities|Text|ToText(Integer) _output_get_2)))
  (if (== (Variables|Default|GetTimeToGameOverSecond) 0)
    (if (== (Variables|Default|GetTimeToGameOverMinute) 0)
      (return))))

(fn SetTimer
  (Rendering|Components|TextRender|SetText (Variables|Default|GetSeconds) (Utilities|Text|ToText(Integer) (Variables|Default|GetTimeToGameOverSecond)))
  (Rendering|Components|TextRender|SetText (Variables|Default|GetMinutes) (Utilities|Text|ToText(Integer) (Variables|Default|GetTimeToGameOverMinute))))